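; Animation modifier that bakes the root bone's yaw rotation into a named float curve on an animation sequence.
; On apply, it replaces any existing curve of that name, then samples the root bone pose on each frame with root motion extraction and writes the yaw as a key at that frame's time.
; On revert, it removes the curve.
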(event EventOnApply
  (params (AnimationSequence :type Anim%20Sequence%20Object%20Reference))
  (bind _output_get (Variables|Default|SetAnimation%20Sequence AnimationSequence))
  (bind _returnvalue (Class|AnimationBlueprintLibrary|DoesCurveExist _output_get (Variables|Default|GetCurveName) "RCT_Float"))
  (if _returnvalue
    (Class|AnimationBlueprintLibrary|RemoveCurve (Variables|Default|GetAnimation%20Sequence) (Variables|Default|GetCurveName) false))
  (Class|AnimationBlueprintLibrary|AddCurve (Variables|Default|GetAnimation%20Sequence) (Variables|Default|GetCurveName) "RCT_Float" false)
  (for _index (range 0 (Class|AnimationBlueprintLibrary|GetNumFrames (Variables|Default|GetAnimation%20Sequence)))
    (Class|AnimationBlueprintLibrary|AddFloatCurveKey (Variables|Default|GetAnimation%20Sequence) (Variables|Default|GetCurveName) (Class|AnimationBlueprintLibrary|GetTimeatFrame (Variables|Default|GetAnimation%20Sequence) _index) (.yaw (.rotation (Class|AnimationBlueprintLibrary|GetBonePoseforFrame (Variables|Default|GetAnimation%20Sequence) "root" _index true))))))

(event EventOnRevert
  (params (AnimationSequence :type Anim%20Sequence%20Object%20Reference))
  (bind _output_get (Variables|Default|SetAnimation%20Sequence AnimationSequence))
  (bind _returnvalue (Class|AnimationBlueprintLibrary|DoesCurveExist _output_get (Variables|Default|GetCurveName) "RCT_Float"))
  (if _returnvalue
    (Class|AnimationBlueprintLibrary|RemoveCurve (Variables|Default|GetAnimation%20Sequence) (Variables|Default|GetCurveName) false)))