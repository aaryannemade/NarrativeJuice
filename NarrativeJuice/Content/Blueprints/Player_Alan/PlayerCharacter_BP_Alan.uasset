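; Player character Blueprint with camera-relative movement and mouse or gamepad look, tracking locomotion start and stop states.
; Tick smoothly rotates the actor toward input direction relative to control yaw while ShouldRotate is set; this file only clears that flag.
; It records StartDirection as movement begins and predicts StopLocation once per stop from CharacterMovement physics.
; Debug prints, a stop-location sphere and a forward line trace visualise the results.
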(event EventTick
  (params (DeltaSeconds :type Float%20%28single-precision%29))
  (bind _returnvalue (Transformation|GetActorLocation))
  (bind _charactermovement (Variables|Character|GetCharacterMovement))
  (Utilities|FlowControl|Sequence
    (:then_0
      (|SetIsMoving))
    (:then_1
      (if (and (Variables|Default|GetMovementInput) (Variables|Default|GetShouldRotate))
        (Variables|Default|SetDesiredRotation (CallFunction|CalculateDesiredRotation))
        (Transformation|SetActorRotation (Math|Interpolation|RInterpTo (Transformation|GetActorRotation) (Variables|Default|GetDesiredRotation) (Utilities|Time|GetWorldDeltaSeconds) 3.0))))
    (:then_2
      (|SetStartDirection))
    (:then_3
      (|SetMovinglastFrame))
    (:then_4
      (if (CallFunction|GetMovementInput)
        (Variables|Default|SetStopped false)
        (Utilities|FlowControl|DoOnce false
          (:Completed
            (Variables|Default|SetHasMoved true)))
        (elif (Variables|Default|GetHasMoved)
          (Variables|Default|SetStopped true)
          (else
            (Variables|Default|SetStopped false)))))
    (:then_5
      (if (Variables|Default|GetStopped)
        (Utilities|FlowControl|DoOnce false :!label _label
          (:Completed
            (bind _outstoplocation (Class|DistanceMatchingPluginBPLibrary|PredictStopLocation (Transformation|GetActorLocation) (Transformation|GetVelocity) (Pawn|Components|CharacterMovement|GetCurrentAcceleration _charactermovement) (Variables|/Script/Engine.CharacterMovementComponent|GetGroundFriction _charactermovement) (Variables|/Script/Engine.CharacterMovementComponent|GetBrakingDecelerationWalking _charactermovement) (Utilities|Time|GetWorldDeltaSeconds) 1000))
            (bind _output_get (Variables|Default|SetStopLocation _outstoplocation))
            (Rendering|Debug|DrawDebugSphere _output_get 25.0 12 "(R=1.000000,G=0.000000,B=0.265757,A=1.000000)" 5.0 1.0)
            (Development|PrintString (Utilities|String|Append "Distance to stop: " (Utilities|String|ToString(Float) (Math|Vector|VectorLength (- _output_get (Transformation|GetActorLocation)))) "cm"))))
        (else
          (goto _label Reset))))
    (:then_6
      (Collision|LineTraceByChannel _returnvalue (+ _returnvalue (* (Transformation|GetActorForwardVector) 1e+02)) "TraceTypeQuery1" false 0 "ForOneFrame"))))

(event Input|AxisEvents|InputAxisMoveForward/Backward
  (params (AxisValue :type Float%20%28single-precision%29))
  ;[1 1 1] Character Movement
  (bind _output_get (Variables|Default|SetInputX AxisValue))
  (Pawn|Input|AddMovementInput (Math|Vector|GetForwardVector (Math|Rotator|MakeRotator 0.0 0.0 (.yaw (Pawn|GetControlRotation :!class /Script/Engine.Pawn)))) _output_get false))

(event Input|AxisEvents|InputAxisMoveRight/Left
  (params (AxisValue :type Float%20%28single-precision%29))
  ;[1 1 1] Character Movement
  (bind _output_get (Variables|Default|SetInputY AxisValue))
  (Pawn|Input|AddMovementInput (Math|Vector|GetRightVector (Math|Rotator|MakeRotator 0.0 0.0 (.yaw (Pawn|GetControlRotation :!class /Script/Engine.Pawn)))) _output_get false))

(event Input|AxisEvents|InputAxisTurnRight/LeftMouse
  (params (AxisValue :type Float%20%28single-precision%29))
  ;[1 1 1] Camera Control - Mouse
  (Pawn|Input|AddControllerYawInput AxisValue))

(event Input|AxisEvents|InputAxisLookUp/DownMouse
  (params (AxisValue :type Float%20%28single-precision%29))
  ;[1 1 1] Camera Control - Mouse
  (Pawn|Input|AddControllerPitchInput AxisValue))

(event Input|AxisEvents|InputAxisTurnRight/LeftGamepad
  (params (AxisValue :type Float%20%28single-precision%29))
  ;[1 1 1] Camera Control - Gamepad
  (Pawn|Input|AddControllerYawInput (* AxisValue (Variables|Default|GetGamepadCameraSensitivity) (Utilities|Time|GetWorldDeltaSeconds))))

(event Input|AxisEvents|InputAxisLookUp/DownGamepad
  (params (AxisValue :type Float%20%28single-precision%29))
  ;[1 1 1] Camera Control - Gamepad
  (Pawn|Input|AddControllerPitchInput (* AxisValue (Variables|Default|GetGamepadCameraSensitivity) (Utilities|Time|GetWorldDeltaSeconds))))

(fn ConstructionScript)

(fn CalculateDesiredRotation
  (return (Math|Rotator|Delta(Rotator) (Math|Rotator|MakeRotator 0.0 0.0 (.yaw (Pawn|GetControlRotation :!class /Script/Engine.Pawn))) (Math|Rotator|MakeRotator 0.0 0.0 (.yaw (Math|Conversions|RotationFromXVector (Math|Vector|MakeVector (Variables|Default|GetInputX) (* (Variables|Default|GetInputY) -1.0) 0.0)))))))

(fn StartedMoving
  (return (and (Variables|Default|GetMovementInput) (not (Variables|Default|GetWasMovingLastFrame)))))

(fn GetMovementInput
  (return (or (!= (Input|AxisValues|GetMoveForward/Backward) 0.0) (!= (Input|AxisValues|GetMoveRight/Left) 0.0))))