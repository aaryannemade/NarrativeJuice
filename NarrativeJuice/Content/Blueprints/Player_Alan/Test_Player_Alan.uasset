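; Test player character for Alan that hands parkour behavior to a ParkourMovement component.
; It initializes the component with itself on BeginPlay, then forwards movement mode changes and landing events to it.
; The Jump input runs the standard character jump and also notifies the component on press, while release only stops the jump.
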(event EventBeginPlay
  (Default|Initialize (Variables|Default|GetParkourMovement) self))

(event EventOnMovementModeChanged
  (params (PrevMovementMode :type EMovementMode%20Enum :default "MOVE_None") (NewMovementMode :type EMovementMode%20Enum :default "MOVE_None") (PrevCustomMode :type Byte :default 0) (NewCustomMode :type Byte :default 0))
  (Default|MovementChanged (Variables|Default|GetParkourMovement) PrevMovementMode NewMovementMode))

(event EventOnLanded
  (params (Hit :type Hit%20Result%20Structure%20%28by%20ref%29))
  (Default|LandEvent (Variables|Default|GetParkourMovement)))

(event Input|ActionEvents|InputActionJump
  (params (Key :type Key%20Structure))
  (:Pressed
    (Character|Jump)
    (Default|JumpEvent (Variables|Default|GetParkourMovement)))
  (:Released
    (Character|StopJumping)))

(fn ConstructionScript)