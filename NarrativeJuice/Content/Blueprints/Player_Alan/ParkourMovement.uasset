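; Parkour movement logic for a character, adding side wall runs, vertical wall runs, ledge grabs, mantles and jumps off walls or ledges.
; A looping timer drives gated updates and camera roll, with gates opened and closed by jumping, landing, falling and cooldown timers.
; Traces detect walls and ledges, launches propel runs and jumps, and interpolation moves mantles.
; A parkour mode enum tracks state and restores gravity and movement mode on exit.
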(event Custom|Initialize
  (params (Character :type Character%20Object%20Reference))
  (bind _output_get (Variables|Default|SetCharacter Character))
  (bind _output_get_2 (Variables|Components|SetCharacter%20Movement (Variables|/Script/Engine.Character|GetCharacterMovement _output_get)))
  (Variables|Default|SetDefaultGravity (Variables|/Script/Engine.CharacterMovementComponent|GetGravityScale _output_get_2))
  (Utilities|Time|SetTimerbyEvent (delegate Custom|WallRunUpdate%20Event) 0.01 true))

(event Custom|Jump%20Event
  (if (Utilities|Enum|Equal(Enum) (Variables|Default|GetCurrentParkourMovementMode) "NewEnumerator0")
    (if (not (AI|Components|NavMovement|IsFalling (Variables|Components|GetCharacter%20Movement)))
      (CallFunction|OpenGates))
    (else
      (WallRun|WallRunJump)
      (CallFunction|LedgeGrapJump))))

(event Custom|WallRunUpdate%20Event
  (Utilities|FlowControl|Sequence
    (:then_0
      (|WallRun))
    (:then_1
      (|VerticalWallRun))
    (:then_2
      (|Mantle))
    (:then_3
      (CallFunction|CameraTick))))

(event Custom|MovementChanged
  (params (PrevMovementMode :type EMovementMode%20Enum :default "MOVE_None") (NewMovementMode :type EMovementMode%20Enum :default "MOVE_None"))
  (Utilities|IsValid (Variables|Components|GetCharacter%20Movement)
    (:Is%20Valid
      (Variables|Default|SetPrevMovementMode PrevMovementMode)
      (Variables|Default|SetCurrentMovementMode NewMovementMode)
      (|OpenGatesNode))))

(event Custom|ParkourMovementChanged
  (params (PrevParkourMovementMode :type E_ParkourMovement%20Enum :default "NewEnumerator0") (NewParkourMovementMode :type E_ParkourMovement%20Enum :default "NewEnumerator0"))
  (Variables|Default|SetPrevParkourMovementMode PrevParkourMovementMode)
  (Variables|Default|SetCurrentParkourMovementMode NewParkourMovementMode)
  (CallFunction|ResetMovement))

(event Custom|Land%20Event
  (WallRun|WallRunEnd 0.0)
  (CallFunction|VerticalWallRunEnd 0.0)
  (CallFunction|CloseGates))

(fn WallRunUpdate
  (if (Utilities|CanWallRun)
    (bind _onwall (WallRun|WallRunMovement (Transformation|GetActorLocation (Variables|Default|GetCharacter)) (.Right (Utilities|WallRunEndVectors)) -1.0)) ; Right
    (if _onwall
      (CallFunction|SetParkourMovementMode "NewEnumerator2")
      (Variables|/Script/Engine.CharacterMovementComponent|SetGravityScale (Variables|Components|GetCharacter%20Movement) (Math|Interpolation|FInterpTo (Variables|/Script/Engine.CharacterMovementComponent|GetGravityScale (Variables|Components|GetCharacter%20Movement)) (Variables|WallRun|GetWallRunTargetGravity) (Utilities|Time|GetWorldDeltaSeconds) 1e+01) :!label _label)
      (elif (Utilities|Enum|Equal(Enum) (Variables|Default|GetCurrentParkourMovementMode) "NewEnumerator2")
        (WallRun|WallRunEnd 0.5)
        (else
          (bind _onwall_2 (WallRun|WallRunMovement (Transformation|GetActorLocation (Variables|Default|GetCharacter)) (.Left (Utilities|WallRunEndVectors)) 1.0)) ; Left
          (if _onwall_2
            (CallFunction|SetParkourMovementMode "NewEnumerator1")
            (goto _label)
            (else
              (WallRun|WallRunEnd 0.5))))))
    (else
      (WallRun|WallRunEnd 1.0))))

(fn WallRunMovement
  (params (Start :type Vector) (End :type Vector) (WallRunDirection :type Float%20%28double-precision%29))
  (bind _outhit (Collision|LineTraceByChannel Start End "TraceTypeQuery1" false 0 "None"))
  (if (.bblockinghit _outhit)
    (Variables|WallRun|SetWallRunNormal (.normal _outhit))
    (if (and (AI|Components|NavMovement|IsFalling (Variables|Components|GetCharacter%20Movement)) (Utilities|ValidWallRunVector? (.normal _outhit)))
      (Character|LaunchCharacter (Variables|Default|GetCharacter) (* (Math|Vector|CrossProduct (Variables|WallRun|GetWallRunNormal) "0, 0,1.000000") (* WallRunDirection (Variables|WallRun|GetWallRunSpeed))) true (not (Variables|WallRun|GetWallRunGravity)))
      (return true)
      (else
        (return false)))
    (else
      (return false))))

(fn WallRunJump
  (bind _wallrunjumpoffforce (Variables|WallRun|GetWallRunJumpOffForce))
  (bind _wallrunnormal (Variables|WallRun|GetWallRunNormal))
  (if (Utilities|WallRunning?)
    (WallRun|WallRunEnd 0.35)
    (Character|LaunchCharacter (Variables|Default|GetCharacter) (Math|Vector|MakeVector (* _wallrunjumpoffforce (.x _wallrunnormal)) (* _wallrunjumpoffforce (.y _wallrunnormal)) (Variables|WallRun|GetWallRunJumpHeight)) false true)))

(fn WallRunEnd
  (params (ResetTime :type Float%20%28double-precision%29))
  (if (Utilities|WallRunning?)
    (bind _change (CallFunction|SetParkourMovementMode "NewEnumerator0"))
    (if _change
      (CallFunction|CloseWallRunGate)
      (Utilities|Time|SetTimerbyFunctionName 0 "OpenWallRunGate" ResetTime))))

(fn CameraTick
  (switch Utilities|FlowControl|Switch|SwitchonE_ParkourMovement (Variables|Default|GetCurrentParkourMovementMode)
    (:NewEnumerator0
      (CallFunction|CameraTilt 0.0 :!label _label))
    (:NewEnumerator1
      (CallFunction|CameraTilt 15.0))
    (:NewEnumerator2
      (CallFunction|CameraTilt -15.0))
    (:NewEnumerator3
      (goto _label))
    (:NewEnumerator4
      (goto _label))
    (:NewEnumerator5
      (goto _label))))

(fn CameraTilt
  (params (Target%20X%20 :type Float%20%28double-precision%29))
  (bind _character (Variables|Default|GetCharacter))
  (bind _returnvalue (Pawn|GetController _character))
  (bind _returnvalue_2 (Pawn|GetControlRotation _returnvalue :!class /Script/Engine.Controller))
  (bind (_roll _pitch _yaw) (Math|Rotator|BreakRotator _returnvalue_2))
  (Pawn|SetControlRotation (Pawn|GetController (Variables|Default|GetCharacter)) (Math|Interpolation|RInterpTo _returnvalue_2 (Math|Rotator|MakeRotator Target%20X%20 _pitch _yaw) (Utilities|Time|GetWorldDeltaSeconds) 1e+01)))

(fn ResetMovement
  (if (Utilities|Enum|Equal(Enum) (Variables|Default|GetCurrentParkourMovementMode) "NewEnumerator0")
    (Variables|/Script/Engine.CharacterMovementComponent|SetGravityScale (Variables|Components|GetCharacter%20Movement) (Variables|Default|GetDefaultGravity))
    (Pawn|Components|CharacterMovement|SetMovementMode (Variables|Components|GetCharacter%20Movement) (Utilities|Select :Index (Variables|Default|GetPrevParkourMovementMode) :NewEnumerator0 "MOVE_Falling" :NewEnumerator1 "MOVE_Falling" :NewEnumerator2 "MOVE_Falling" :NewEnumerator3 "MOVE_Falling" :NewEnumerator4 "MOVE_Falling" :NewEnumerator5 "MOVE_Walking") 0)))

(fn SetParkourMovementMode
  (params (New%20Mode :type E_ParkourMovement%20Enum :default "NewEnumerator0"))
  (if (Utilities|Enum|Equal(Enum) New%20Mode (Variables|Default|GetCurrentParkourMovementMode))
    (return false)
    (else
      (CallFunction|ParkourMovementChanged (Variables|Default|GetCurrentParkourMovementMode) New%20Mode)
      (return true))))

(fn VerticalWallRunUpdate
  (bind (_eyes _feet) (Utilities|MantleVectors))
  (if (Utilities|CanVerticalWallRun)
    (bind (_outhit _returnvalue) (Collision|CapsuleTraceByChannel _eyes _feet 2e+01 1e+01 "TraceTypeQuery1" false 0 "None"))
    (if _returnvalue
      (Variables|Default|SetMantleTraceDistance (.Distance (Collision|BreakHitResult _outhit)))
      (if (Class|CharacterMovementComponent|IsWalkable (Variables|Components|GetCharacter%20Movement) _outhit)
        (Variables|Default|SetMantlePosition (+ (.ImpactPoint (Collision|BreakHitResult _outhit)) (Math|Vector|MakeVector 0.0 0.0 (Variables|/Script/Engine.CapsuleComponent|GetCapsuleHalfHeight (Variables|/Script/Engine.Character|GetCapsuleComponent (Variables|Default|GetCharacter))))))
        (CallFunction|CloseVerticalWallRunGate)
        (|LedgeGrab)
        (if (Utilities|QuickMantle)
          (CallFunction|OpenMantleCheckGate)
          (else
            (Utilities|Time|SetTimerbyFunctionName 0 "OpenMantleCheckGate" 0.25)))
        (else
          (CallFunction|VerticalWallRunMovement)))
      (else
        (CallFunction|VerticalWallRunMovement)))
    (else
      (CallFunction|VerticalWallRunEnd 0.35))))

(fn VerticalWallRunEnd
  (params (Reset%20Time :type Float%20%28double-precision%29))
  (bind _currentparkourmovementmode (Variables|Default|GetCurrentParkourMovementMode))
  (if (Math|Boolean|ORBoolean (Utilities|Enum|Equal(Enum) _currentparkourmovementmode "NewEnumerator4") (Utilities|Enum|Equal(Enum) _currentparkourmovementmode "NewEnumerator3") (Utilities|Enum|Equal(Enum) _currentparkourmovementmode "NewEnumerator5"))
    (bind _change (CallFunction|SetParkourMovementMode "NewEnumerator0"))
    (if _change
      (CallFunction|CloseVerticalWallRunGate)
      (CallFunction|CloseMantleCheckGate)
      (Utilities|Time|SetTimerbyFunctionName 0 "OpenVerticalWallRunGate" Reset%20Time))))

(fn VerticalWallRunMovement
  (bind _feet (Utilities|MantleVectors))
  (bind (_outhit _returnvalue) (Collision|LineTraceByChannel _feet (+ _feet (* (Transformation|GetActorForwardVector (Variables|Default|GetCharacter)) 5e+01)) "TraceTypeQuery1" false 0 "None"))
  (if (and (> (Utilities|ForwardInput) 0.0) _returnvalue)
    (Variables|VerticalWallRun|SetVerticalWallRunNormal (.Normal (Collision|BreakHitResult _outhit)))
    (CallFunction|SetParkourMovementMode "NewEnumerator3")
    (Character|LaunchCharacter (Variables|Default|GetCharacter) (Math|Vector|MakeVector (.x (* (Variables|VerticalWallRun|GetVerticalWallRunNormal) -6e+02)) (.y (* (Variables|VerticalWallRun|GetVerticalWallRunNormal) -6e+02)) (Variables|VerticalWallRun|GetVerticalWallRunSpeed)) true true)
    (else
      (CallFunction|VerticalWallRunEnd 0.35))))

(fn MantleMovement
  (bind _character (Variables|Default|GetCharacter))
  (bind _character_2 (Variables|Default|GetCharacter))
  (bind _mantleposition (Variables|Default|GetMantlePosition))
  (bind _returnvalue (Pawn|GetController _character))
  (bind _returnvalue_2 (Transformation|GetActorLocation _character_2))
  (Pawn|SetControlRotation _returnvalue (Math|Interpolation|RInterpTo (Pawn|GetControlRotation _returnvalue :!class /Script/Engine.Controller) (Math|Rotator|FindLookatRotation (Math|Vector|MakeVector (.x _returnvalue_2) (.y _returnvalue_2) 0.0) (Math|Vector|MakeVector (.x _mantleposition) (.y _mantleposition) 0.0)) (Utilities|Time|GetWorldDeltaSeconds) 7.0))
  (Transformation|SetActorLocation (Variables|Default|GetCharacter) (Math|Interpolation|VInterpTo (Transformation|GetActorLocation (Variables|Default|GetCharacter)) (Variables|Default|GetMantlePosition) (Utilities|Time|GetWorldDeltaSeconds) (select (Utilities|QuickMantle) (Variables|Default|GetQuickMatleSpeed) (Variables|Default|GetMantleSpeed))) false false)
  (if (< (Math|Vector|Distance(Vector) (Transformation|GetActorLocation (Variables|Default|GetCharacter)) (Variables|Default|GetMantlePosition)) 8.0)
    (CallFunction|VerticalWallRunEnd 0.5)))

(fn OpenGates
  (CallFunction|OpenWallRunGate)
  (CallFunction|OpenVerticalWallRunGate))

(fn CloseGates
  (CallFunction|CloseWallRunGate)
  (CallFunction|CloseVerticalWallRunGate))

(fn LedgeGrapJump
  (bind _currentparkourmovementmode (Variables|Default|GetCurrentParkourMovementMode))
  (bind _verticalwallrunnormal (Variables|VerticalWallRun|GetVerticalWallRunNormal))
  (if (Math|Boolean|ORBoolean (Utilities|Enum|Equal(Enum) _currentparkourmovementmode "NewEnumerator4") (Utilities|Enum|Equal(Enum) _currentparkourmovementmode "NewEnumerator3") (Utilities|Enum|Equal(Enum) _currentparkourmovementmode "NewEnumerator5"))
    (CallFunction|VerticalWallRunEnd 0.35)
    (Character|LaunchCharacter (Variables|Default|GetCharacter) (Math|Vector|MakeVector (* (.x _verticalwallrunnormal) (Variables|Default|GetLedgeGrabJumpOffForce)) (* (.y _verticalwallrunnormal) (Variables|Default|GetLedgeGrabJumpOffForce)) (Variables|Default|GetLedgeGrabJumpHeight)) false true)))

(event Custom|OpenMantleCheckGate
  (Utilities|FlowControl|Gate true) ; enters at Open
)

(event Custom|CloseMantleCheckGate
  (Utilities|FlowControl|Gate true) ; enters at Close
)

(event Custom|OpenMantleGate
  (Utilities|FlowControl|Gate true) ; enters at Open
)

(event Custom|CloseMantleGate
  (Utilities|FlowControl|Gate true) ; enters at Close
)

(event Custom|MantleCheck
  (if (Utilities|CanMantle)
    (CallFunction|MantleStart)))

(event Custom|MantleStart
  (bind _change (CallFunction|SetParkourMovementMode "NewEnumerator5"))
  (if _change
    (CallFunction|CloseMantleCheckGate)
    (CallFunction|OpenMantleGate)))

(event Custom|OpenWallRunGate
  (Utilities|FlowControl|Gate true) ; enters at Open
)

(event Custom|CloseWallRunGate
  (Utilities|FlowControl|Gate true) ; enters at Close
)

(event Custom|OpenVerticalWallRunGate
  (Utilities|FlowControl|Gate true) ; enters at Open
)

(event Custom|CloseVerticalWallRunGate
  (CallFunction|CloseMantleGate)
  (Utilities|FlowControl|Gate true) ; enters at Close
)